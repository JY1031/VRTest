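; VR player component that provides a right-hand laser aim and fire action for BP_VRPlayerPawn.
; Each tick it line-traces forward from the hand, caching the hit and feeding the endpoints to the pawn's Niagara beam.
; A Niagara crosshair sits at the trace end, oriented to the last impact normal.
; On Fire, a cached hit spawns an explosion and pushes physics-simulating components along the aim direction with mass-scaled force.
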(event `self.ReceiveBeginPlay`
  (bind _asbp_vrplayer_pawn (cast `/Game/Blueprints/BP_VRPlayerPawn` (`self.GetOwner`)))
  (bind _output_get (set `self.me` _asbp_vrplayer_pawn))
  (set `self.hand` (`/Game/Blueprints/BP_VRPlayerPawn.MannequinHand_Right` _output_get)))

(event `self.ReceiveTick`
  (params (DeltaSeconds :type "Float (single-precision)"))
  (`self.DrawLine`))

(event `Fire`
  (bind _hitcomp (`self.hitComp`))
  (if (`self.bHit`)
    (`GameplayStatics.SpawnEmitterAtLocation` "/Game/StarterContent/Particles/P_Explosion.P_Explosion" (`self.end`))
    (if (`SceneComponent.IsSimulatingPhysics` _hitcomp "None")
      (`PrimitiveComponent.AddForce` _hitcomp (* (* (`KismetMathLibrary.Normal` (- (`self.end`) (`self.start`))) (`PrimitiveComponent.GetMass` _hitcomp)) 2000.0) "None" true))))

(fn `DrawLine`
  (locals (normal :type "Vector Structure"))
  (bind _hand (`self.hand`))
  (bind _returnvalue (`SceneComponent.K2_GetComponentLocation` _hand))
  (`|ExecutionSequence`
    (:`then_0`
      (bind _output_get (set `self.start` _returnvalue))
      (bind _output_get_2 (set `self.end` (+ _returnvalue (* (`SceneComponent.GetForwardVector` _hand) (`self.dist`)))))
      (bind (_outhit _returnvalue_2) (`KismetSystemLibrary.LineTraceSingleForObjects` _output_get _output_get_2 (`|MakeArray` "ObjectTypeQuery1" "ObjectTypeQuery2" "ObjectTypeQuery4" :!type "EObjectTypeQuery Enum") false (`|MakeArray` (`self.me`) :!type "Actor Object Reference") "None" true (struct :`R` 1.0 :`A` 1.0) (struct :`G` 1.0 :`A` 1.0) 0.2))
      (bind _output_get_3 (set `self.bHit` _returnvalue_2))
      (if _output_get_3
        (bind (_bblockinghit _binitialoverlap _time _distance _location _impactpoint _normal _impactnormal _physmat _hitactor _hitcomponent) (`GameplayStatics.BreakHitResult` _outhit))
        (set `self.end` _impactpoint)
        (set `self.hitActor` _hitactor)
        (set `local.normal` _impactnormal)
        (set `self.hitComp` _hitcomponent)))
    (:`then_1`
      (`NiagaraDataInterfaceArrayFunctionLibrary.SetNiagaraArrayVector` (`/Game/Blueprints/BP_VRPlayerPawn.FireTraceNiagaraSystem` (`self.me`)) "User.PointArray" (`|MakeArray` (`self.start`) (`self.end`)))
      (`SceneComponent.K2_SetWorldLocationAndRotation` (`/Game/Blueprints/BP_VRPlayerPawn.FireCrosshairNiagaraSystem` (`self.me`)) (`self.end`) (`KismetMathLibrary.MakeRotFromZX` (`local.normal`) (`SceneComponent.GetForwardVector` (`/Game/Blueprints/BP_VRPlayerPawn.FireCrosshairNiagaraSystem` (`self.me`)))) false false))))