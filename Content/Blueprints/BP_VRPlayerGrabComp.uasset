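; Actor component for the VR player pawn that lets the right hand grab and throw physics objects.
; On grab, a line trace from the hand finds a physics body, disables its simulation and gravity, and attaches it to the hand socket.
; On release, it detaches, restores physics, and adds the motion controller's angular velocity plus its linear velocity scaled by force and object mass.
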(event `self.ReceiveBeginPlay`
  (bind _asbp_vrplayer_pawn (cast `/Game/Blueprints/BP_VRPlayerPawn` (`self.GetOwner`)))
  (bind _output_get (set `self.me` _asbp_vrplayer_pawn))
  (set `self.hand` (`/Game/Blueprints/BP_VRPlayerPawn.MannequinHand_Right` _output_get))
  (set `self.controller` (`/Game/Blueprints/BP_VRPlayerPawn.RightMotionController` _output_get)))

(event `GrabPressed`
  (bind _hitcomp (`self.hitComp`))
  (bind _hand (`self.hand`))
  (bind _returnvalue (`SceneComponent.K2_GetComponentLocation` _hand))
  (bind (_outhit _returnvalue_2) (`KismetSystemLibrary.LineTraceSingleForObjects` _returnvalue (+ _returnvalue (* (`SceneComponent.GetForwardVector` _hand) (`self.dist`))) (`|MakeArray` "ObjectTypeQuery4" :!type "EObjectTypeQuery Enum") false (`|MakeArray` (`self.me`) :!type "Actor Object Reference")))
  (bind _output_get (set `self.bHit` _returnvalue_2))
  (if _output_get
    (bind (_bblockinghit _binitialoverlap _time _distance _location _impactpoint _normal _impactnormal _physmat _hitactor _hitcomponent) (`GameplayStatics.BreakHitResult` _outhit))
    (set `self.hitComp` _hitcomponent)
    (set `self.hitActor` _hitactor)
    (`PrimitiveComponent.SetSimulatePhysics` _hitcomp false)
    (`PrimitiveComponent.SetEnableGravity` _hitcomp false)
    (`Actor.K2_AttachToComponent` (`self.hitActor`) (`self.hand`) "hand_rSocket" "SnapToTarget" "KeepWorld" "KeepWorld" true)))

(event `GrabReleased`
  (bind _hitcomp (`self.hitComp`))
  (if (`self.bHit`)
    (`Actor.K2_DetachFromActor` (`self.hitActor`) "KeepWorld" "KeepWorld" "KeepWorld")
    (set `self.bHit` false)
    (`PrimitiveComponent.SetSimulatePhysics` _hitcomp true)
    (`PrimitiveComponent.SetEnableGravity` _hitcomp true)
    (bind _returnvalue (`PrimitiveComponent.GetPhysicsLinearVelocity` (`self.controller`) "None"))
    (`PrimitiveComponent.SetPhysicsLinearVelocity` (`self.hitComp`) (* _returnvalue (* (`self.force`) (`PrimitiveComponent.GetMass` (`self.hitComp`)))) true "None")
    (`PrimitiveComponent.SetPhysicsAngularVelocityInDegrees` (`self.hitComp`) (`PrimitiveComponent.GetPhysicsAngularVelocityInDegrees` (`self.controller`) "None") true "None")))