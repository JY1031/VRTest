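; BP_VRPlayerMoveComp is a component that gives its owning VR player thumbstick locomotion, with smooth movement and turning.
; BeginPlay caches the owner, then LeftX and LeftY axis events feed Translate, which offsets location along the owner's right and forward vectors.
; RightX applies world yaw rotation.
; Both motions scale by speed variables and delta time, and translation sets location directly without sweeping for collision.
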(event `self.ReceiveBeginPlay`
  (set `self.me` (`self.GetOwner`)))

(event `LeftX`
  (params (AxisValue :type "Float (double-precision)"))
  (`self.Translate` (`Actor.GetActorRightVector` (`self.me`)) AxisValue))

(event `LeftY`
  (params (AxisValue :type "Float (double-precision)"))
  (`self.Translate` (`Actor.GetActorForwardVector` (`self.me`)) AxisValue))

(event `RightX`
  (params (AxisValue :type "Float (double-precision)"))
  (`Actor.K2_AddActorWorldRotation` (`self.me`) (`KismetMathLibrary.MakeRotator` 0.0 0.0 (* AxisValue (`GameplayStatics.GetWorldDeltaSeconds`) (`self.rotSpeed`))) false false))

(fn `Translate`
  (params (Direction :type "Vector Structure") (AxisValue :type "Float (double-precision)"))
  (`Actor.K2_SetActorLocation` (`self.me`) (+ (`Actor.K2_GetActorLocation` (`self.me`)) (* (* Direction (* AxisValue (`self.moveSpeed`))) (`GameplayStatics.GetWorldDeltaSeconds`))) false false))