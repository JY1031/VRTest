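; VR player pawn that sets floor tracking origin when a headset is enabled and routes motion controller input to gameplay components.
; Stick axes feed a movement component, left trigger and X drive arc and line teleport in a teleport component, and A fires through a fire component.
; Grip axes set GripValue on each mannequin hand's animation instance, while text renders display stick values.
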(event `self.ReceiveBeginPlay`
  (if (`HeadMountedDisplayFunctionLibrary.IsHeadMountedDisplayEnabled`)
    (`HeadMountedDisplayFunctionLibrary.SetTrackingOrigin` "Floor")))

(event `InputAxis|GrabAxisLeft`
  (params (AxisValue :type "Float (single-precision)"))
  (bind _asabp_vrhand (cast `/Game/Blueprints/ABP_VRHand` (`SkeletalMeshComponent.GetAnimInstance` (`self.MannequinHand_Left`))))
  (set `/Game/Blueprints/ABP_VRHand.GripValue` AxisValue _asabp_vrhand))

(event `InputAxis|GrabAxisRight`
  (params (AxisValue :type "Float (single-precision)"))
  (bind _asabp_vrhand (cast `/Game/Blueprints/ABP_VRHand` (`SkeletalMeshComponent.GetAnimInstance` (`self.MannequinHand_Right`))))
  (set `/Game/Blueprints/ABP_VRHand.GripValue` AxisValue _asabp_vrhand))

(event `InputAxis|MovementAxisLeft_X`
  (params (AxisValue :type "Float (single-precision)"))
  (`/Game/Blueprints/BP_VRPlayerMoveComp.LeftX` (`self.BP_VRPlayerMoveComp`) AxisValue)
  (bind _output_get (set `self.LeftX` AxisValue))
  (`TextRenderComponent.K2_SetText` (`self.LeftTextRender`) (`KismetTextLibrary.Conv_StringToText` (`KismetStringLibrary.Concat_StrStr` (`KismetStringLibrary.Conv_DoubleToString` _output_get) " \n" (`KismetStringLibrary.Conv_DoubleToString` (stale `InputAxis|MovementAxisLeft_Y` _output_get)))) :!label _label))

(event `InputAxis|MovementAxisLeft_Y`
  (params (AxisValue :type "Float (single-precision)"))
  (`/Game/Blueprints/BP_VRPlayerMoveComp.LeftY` (`self.BP_VRPlayerMoveComp`) AxisValue)
  (bind _output_get (set `self.LeftY` AxisValue))
  (goto _label))

(event `InputAxis|MovementAxisRight_X`
  (params (AxisValue :type "Float (single-precision)"))
  (`/Game/Blueprints/BP_VRPlayerMoveComp.RightX` (`self.BP_VRPlayerMoveComp`) AxisValue)
  (`TextRenderComponent.K2_SetText` (`self.RightTextRender`) (`KismetTextLibrary.Conv_DoubleToText` AxisValue "HalfToEven")))

(event `InputAxis|TriggerAxisLeft`
  (params (AxisValue :type "Float (single-precision)"))
  (`/Game/Blueprints/BP_VRPlayerTeleportComp.ArcTeleport` (`self.BP_VRPlayerTeleportComp`) AxisValue))

(event `InputAction|ButtonX`
  (params (Key :type "Key Structure"))
  (bind _bp_vrplayerteleportcomp (`self.BP_VRPlayerTeleportComp`))
  (:`Pressed`
    (`/Game/Blueprints/BP_VRPlayerTeleportComp.LineTeleportPressed` _bp_vrplayerteleportcomp (`self.MannequinHand_Left`)))
  (:`Released`
    (`/Game/Blueprints/BP_VRPlayerTeleportComp.LineTeleportReleased` _bp_vrplayerteleportcomp)))

(event `InputAction|ButtonA`
  (params (Key :type "Key Structure"))
  (:`Pressed`
    (`/Game/Blueprints/BP_VRPlayerFireComp.Fire` (`self.BP_VRPlayerFireComp`))))

(fn `UserConstructionScript`)